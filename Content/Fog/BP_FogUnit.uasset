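; BP_FogUnit is a fog-of-war unit actor that runs an unfinished vision system every tick.
; VisionSystem writes the actor's location into the PlayerPosition parameter of the C_PlayerPosition material parameter collection.
; It then clears VisionRenderTarget to black and begins canvas drawing on it.
; The DrawTriangle node is unconnected and the draw is never ended, so no vision shape is rendered.
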(event `self.ReceiveTick`
  (params (DeltaSeconds :type "Float (single-precision)"))
  (`parent.ReceiveTick` DeltaSeconds)
  (`self.VisionSystem`))

(fn `UserConstructionScript`
  (`parent.UserConstructionScript`))

(fn `VisionSystem`
  (bind _visionrendertarget (`self.VisionRenderTarget`))
  (`|ExecutionSequence`
    (:`then_0`
      (`KismetMaterialLibrary.SetVectorParameterValue` "/Game/Fog/C_PlayerPosition.C_PlayerPosition" "PlayerPosition" (`KismetMathLibrary.Conv_VectorToLinearColor` (`self.K2_GetActorLocation`))))
    (:`then_1`
      (`KismetRenderingLibrary.ClearRenderTarget2D` _visionrendertarget)
      (`KismetRenderingLibrary.BeginDrawCanvasToRenderTarget` _visionrendertarget))))