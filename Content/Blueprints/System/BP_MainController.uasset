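; BP_MainController is a controller that issues right-click orders to the units in its Units array, RTS style.
; Tick polls the right mouse button, with a DoOnce that resets on release so each press fires a single order.
; On a blocking cursor trace against WorldStatic and Pawn objects, it calls Interaction on every unit with the impact point and hit actor, printing the point for debugging.
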(event `self.ReceiveTick`
  (params (DeltaSeconds :type "Float (single-precision)"))
  (bind _units (`self.Units`))
  (bind (_bblockinghit _binitialoverlap _time _distance _location _impactpoint _normal _impactnormal _physmat _hitactor) (`GameplayStatics.BreakHitResult` (`self.GetHitResultUnderCursorForObjects` (`|MakeArray` "ObjectTypeQuery1" "ObjectTypeQuery3" :!type "EObjectTypeQuery Enum"))))
  (if (`self.IsInputKeyDown` "RightMouseButton")
    (if (`KismetMathLibrary.Conv_IntToBool` (`KismetArrayLibrary.Array_Length` _units))
      (`/Engine/EditorBlueprintResources/StandardMacros.DoOnce` false :!label _label
        (:`Completed`
          (if _bblockinghit
            (for _array_element _units
              (`Unit.Interaction` _array_element _impactpoint _hitactor)
              (`KismetSystemLibrary.PrintString` (`KismetStringLibrary.Conv_VectorToString` _impactpoint)))))))
    (else
      (`|ExecutionSequence`
        (:`then_0`
          (goto _label :!via `Reset`))))))

(fn `UserConstructionScript`)