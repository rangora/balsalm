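; BP_CameraPawn is a camera pawn that pans through the world by keyboard or by screen-edge mouse scrolling.
; Each Tick feeds the forward and right move axes into movement input, then checks the viewport-scaled mouse position against the viewport size.
; MouseMoveOnAxis runs once per screen axis, pushing movement along a fixed world axis when the cursor is within a pixel of either edge.
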(event `self.ReceiveTick`
  (params (DeltaSeconds :type "Float (single-precision)"))
  (bind _returnvalue (`WidgetLayoutLibrary.GetViewportScale`))
  (bind (_returnvalue_x _returnvalue_y) (`KismetMathLibrary.BreakVector2D` (`WidgetLayoutLibrary.GetViewportSize`)))
  ;[1 1 1] Movement by keyboard
  (`|ExecutionSequence`
    (:`then_0`
      (`self.AddMovementInput` (`KismetMathLibrary.MakeVector` (`self.GetInputAxisValue`) (`self.GetInputAxisValue`))))
    (:`then_1`
      ;[1 1 1] Movement by mouse
      (bind _returnvalue_2 (`WidgetLayoutLibrary.GetMousePositionOnViewport`))
      (`self.Mouse Move on Axis` (* (`KismetMathLibrary.BreakVector2D` _returnvalue_2) _returnvalue) _returnvalue_x (0.0 -1.0 0.0))
      (`self.Mouse Move on Axis` (* (`.Y` (`KismetMathLibrary.BreakVector2D` _returnvalue_2)) _returnvalue) _returnvalue_y (1.0 0.0 0.0)))))

(fn `Mouse Move on Axis`
  (params (PositionOnAxis :type "Float (double-precision)") (AxisLength :type "Float (double-precision)") (Axis :type "Vector Structure"))
  (bind _returnvalue (- AxisLength PositionOnAxis))
  (if (< _returnvalue 1.0)
    (`self.AddMovementInput` Axis -1.0)
    (elif (> _returnvalue (- AxisLength 1.0))
      (`self.AddMovementInput` Axis))))

(fn `UserConstructionScript`)