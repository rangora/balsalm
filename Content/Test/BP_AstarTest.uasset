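; BP_AstarTest is a functional test that sends TestUnit to each BP_TestButton in ButtonList, likely to exercise A* pathfinding.
; Each Tick, DoTest calls Interaction on the current button; the Going guard is disconnected, so the call repeats until TurnOn is set.
; An activated button advances the index; completing the list succeeds, an invalid index raises an error, and EndPlay before completion fails.
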(event `self.ReceiveTick`
  (params (DeltaSeconds :type "Float (single-precision)"))
  (bind _result (`self.DoTest` (`self.number`)))
  (`|ExecutionSequence`
    (:`then_0`
      (if (== _result 1)
        (bind _output_get (set `self.number` (+ (`self.number`) 1)))
        (if (== _output_get (`KismetArrayLibrary.Array_Length` (`self.ButtonList`)))
          (`self.FinishTest` "Succeeded" "Test Done")
          (else
            (`KismetSystemLibrary.PrintString` "continue..")))))
    (:`then_1`
      (if (== _result 0)
        _))
    (:`then_2`
      (if (== _result -1)
        (`self.FinishTest` "Error" "Test button index error")))))

(event `self.ReceiveEndPlay`
  (params (EndPlayReason :type "EEndPlayReason Enum" :default "Destroyed"))
  (if (== (`self.number`) (`KismetArrayLibrary.Array_Length` (`self.ButtonList`)))
    (`self.FinishTest` "Succeeded" "Test Done")
    (else
      (`self.FinishTest` "Failed" "Test failed"))))

(fn `DoTest`
  (params (ButtonNumber :type Integer))
  (returns (result :type Integer))
  (locals (Target :type "/Game/Test/BP_TestButton Object Reference"))
  (bind _asbp_test_button (cast `/Game/Test/BP_TestButton` (`|GetArrayItem` (`self.ButtonList`) ButtonNumber) :!pure true))
  (if (`KismetArrayLibrary.Array_IsValidIndex` (`self.ButtonList`) ButtonNumber)
    (if (`KismetSystemLibrary.IsValid` _asbp_test_button)
      (bind _output_get (set `local.Target` _asbp_test_button))
      (set `self.bGoing` true)
      (`Unit.Interaction` (`self.TestUnit`) (`self.K2_GetActorLocation` _output_get) _output_get)
      (if (`/Game/Test/BP_TestButton.bTurnOn` _output_get)
        (set `self.bGoing` false)
        (return 1)
        (else
          (return 0)))
      (else
        (`KismetSystemLibrary.PrintString` "cast failed")))
    (else
      (return -1))))

(fn `UserConstructionScript`)